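; Actor component for Characters that sets jump velocity from a desired jump height and signals when the jump reaches its peak.
; On BeginPlay it caches the owner's capsule and movement component, then derives JumpZVelocity from gravity and gravity scale, with an optional set-once variant.
; Peak events fire either from a per-frame looping timer that detects negative vertical velocity, or after a delay equal to the calculated rise time.
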(event `self.ReceiveBeginPlay`
  (bind _ascharacter (cast `Character` (`self.GetOwner`)))
  (set `self.Character` _ascharacter)
  (set `self.Capsule` (`Character.CapsuleComponent` (`self.Character`)))
  (set `self.CharacterMovement` (`Character.CharacterMovement` (`self.Character`))))

(event `GetJumpPeakEvent`
  (`KismetSystemLibrary.K2_SetTimer` self "ListenJumpPeak" (`GameplayStatics.GetWorldDeltaSeconds`) true))

(event `GetJumpPeakEvent_estimated`
  (`KismetSystemLibrary.Delay` (`self.CalculatePeakTime`))
  (`self.JumpPeakEvent (estimated)`))

(fn `CalculateJumpZVelocity`
  (params (DesiredJumpHeight :type "Float (double-precision)" :default 200.0))
  (returns (JumpZVelocity :type "Float (double-precision)"))
  (bind _charactermovement (`self.CharacterMovement`))
  (return (`KismetMathLibrary.Sqrt` (* 2.0 DesiredJumpHeight (`KismetMathLibrary.Abs` (`MovementComponent.GetGravityZ` _charactermovement)) (`CharacterMovementComponent.GravityScale` _charactermovement)))))

(fn `CalculatePeakTime`
  (returns (PeakTime :type "Float (double-precision)"))
  (bind _charactermovement (`self.CharacterMovement`))
  (return (/ (`CharacterMovementComponent.JumpZVelocity` _charactermovement) (* (`KismetMathLibrary.Abs` (`MovementComponent.GetGravityZ` _charactermovement)) (`CharacterMovementComponent.GravityScale` _charactermovement)))))

(fn `ListenJumpPeak`
  (bind _returnvalue (`PrimitiveComponent.GetPhysicsLinearVelocity` (`self.Capsule`) "None"))
  (if (< (.z _returnvalue) 0.0)
    (`KismetSystemLibrary.K2_ClearTimer` null "ListenJumpPeak")
    (`self.JumpPeakEvent`)))

(fn `SetJumpZVelocity`
  (params (DesiredJumpHeight :type "Float (double-precision)" :default 200.0))
  (set `CharacterMovementComponent.JumpZVelocity` (`self.CalculateJumpZVelocity` DesiredJumpHeight) (`self.CharacterMovement`)))

(fn `SetJumpZVelocityOnce`
  (params (DesiredJumpHeight :type "Float (double-precision)" :default 200.0))
  (`/Engine/EditorBlueprintResources/StandardMacros.DoOnce` false
    (:`Completed`
      (set `CharacterMovementComponent.JumpZVelocity` (`self.CalculateJumpZVelocity` DesiredJumpHeight) (`self.CharacterMovement`)))))